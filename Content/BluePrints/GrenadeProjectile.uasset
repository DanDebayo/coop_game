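; Grenade projectile Blueprint that bounces with a sound on each sphere hit and explodes on a fixed timer.
; BeginPlay spawns the muzzle flash, fire sound and attached trail, then waits out a short delay before calling Explode.
; Explode spawns the explosion effect, deals full radial damage within DamageRadius and destroys the actor.
; A debug sphere drawn after destruction shows the blast radius, and the explosion sound attaches to the explosion emitter.
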(event OnComponentHit(Sphere)
  (params (HitComponent :type Primitive%20Component%20Object%20Reference) (OtherActor :type Actor%20Object%20Reference) (OtherComp :type Primitive%20Component%20Object%20Reference) (NormalImpulse :type Vector :default "0, 0, 0") (Hit :type Hit%20Result%20Structure%20%28by%20ref%29))
  (Audio|SpawnSoundAttached "/Game/SciFiWeapLight/Sound/GrenadeLauncher/Wavs/GL_Bounce03.GL_Bounce03" (Variables|Default|GetSphere) "None" "0, 0, 0" "0, 0, 0" "KeepRelativeOffset" false 1.0 1.0 0.0 0 0))

(event Custom|Explode
  (bind _returnvalue (Transformation|GetActorLocation))
  (bind _returnvalue_2 (Effects|SpawnEmitteratLocation "/Game/SciFiWeapLight/FX/Particles/P_Grenade_Explosion_Dark.P_Grenade_Explosion_Dark" _returnvalue))
  (Game|Damage|ApplyRadialDamage 5e+01 _returnvalue (Variables|Default|GetDamage%20Radius) 0 0 self (Game|GetInstigatorController) true "ECC_Visibility")
  (Actor|DestroyActor)
  (Rendering|Debug|DrawDebugSphere _returnvalue (Variables|Default|GetDamage%20Radius) 12 "(R=0.231705,G=1.000000,B=0.367454,A=1.000000)" 1.0 1.0))

(event EventBeginPlay
  (bind _returnvalue (Effects|SpawnEmitteratLocation "/Game/SciFiWeapLight/FX/Particles/P_Grenade_MuzzleFlash_Dark.P_Grenade_MuzzleFlash_Dark" (Transformation|GetActorLocation)))
  (Audio|SpawnSoundAttached "/Game/SciFiWeapLight/Sound/GrenadeLauncher/Wavs/GL_Fire03.GL_Fire03" _returnvalue "None" "0, 0, 0" "0, 0, 0" "KeepRelativeOffset" false 1.0 1.0 0.0 0 0)
  (Effects|SpawnEmitterAttached "/Game/SciFiWeapLight/FX/Particles/P_Grenade_Trail_Light.P_Grenade_Trail_Light" (Variables|Default|GetSphere) "None")
  (Utilities|FlowControl|Delay 2.0)
  (CallFunction|Explode)
  (Audio|SpawnSoundAttached "/Game/SciFiWeapLight/Sound/GrenadeLauncher/Wavs/GL_Explosion03.GL_Explosion03" (stale Custom|Explode _returnvalue_2) "None" "0, 0, 0" "0, 0, 0" "KeepRelativeOffset" false 1.0 1.0 0.0 0 0))

(fn ConstructionScript)