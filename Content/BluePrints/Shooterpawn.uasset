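; Shooter pawn Blueprint that sets up the local player's HUD.
; On BeginPlay, if the pawn is locally controlled, it creates the Crosshair and HP_Indicate widgets and adds both to the viewport.
; Tick and the construction script are empty, and an unconnected debug print of HPComp's default health never runs.
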(event EventBeginPlay
  (if (Pawn|IsLocallyControlled)
    (Utilities|FlowControl|Sequence
      (:then_0
        (bind _returnvalue (UserInterface|CreateWidget "/Game/UI/Crosshair.Crosshair_C"))
        (UserInterface|Viewport|AddtoViewport _returnvalue 0))
      (:then_1
        (bind _returnvalue_2 (UserInterface|CreateWidget "/Game/UI/HP_Indicate.HP_Indicate_C"))
        (UserInterface|Viewport|AddtoViewport _returnvalue_2 0)))))

(event EventTick
  (params (DeltaSeconds :type Float%20%28single-precision%29)))

(fn ConstructionScript)