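; Rocket projectile Blueprint that explodes on impact or after a fixed lifetime, dealing radial damage.
; BeginPlay spawns a muzzle flash with fire sound and attaches a trail to the collision Sphere.
; The Sphere hit and delay timeout share one path into Explode, then an explosion sound attached to its emitter.
; Explode spawns the effect, applies full damage across the radius with instigator credit, and destroys the actor.
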(event OnComponentHit(Sphere)
  (params (HitComponent :type Primitive%20Component%20Object%20Reference) (OtherActor :type Actor%20Object%20Reference) (OtherComp :type Primitive%20Component%20Object%20Reference) (NormalImpulse :type Vector :default "0, 0, 0") (Hit :type Hit%20Result%20Structure%20%28by%20ref%29))
  (CallFunction|Explode)
  (Audio|SpawnSoundAttached "/Game/SciFiWeapLight/Sound/RocketLauncher/Wavs/RL_Explosion01.RL_Explosion01" (stale Custom|Explode _returnvalue_2) "None" "0, 0, 0" "0, 0, 0" "KeepRelativeOffset" false 1.0 1.0 0.0 0 0))

(event Custom|Explode
  (bind _returnvalue (Transformation|GetActorLocation))
  (bind _returnvalue_2 (Effects|SpawnEmitteratLocation "/Game/SciFiWeapLight/FX/Particles/P_RocketLauncher_Explosion_Light.P_RocketLauncher_Explosion_Light" _returnvalue))
  (Game|Damage|ApplyRadialDamage 1e+02 _returnvalue (Variables|Default|GetDamage%20Radius_0) 0 0 self (Game|GetInstigatorController) true "ECC_Visibility")
  (Actor|DestroyActor))

(event EventBeginPlay
  (bind _returnvalue (Effects|SpawnEmitteratLocation "/Game/SciFiWeapLight/FX/Particles/P_RocketLauncher_MuzzleFlash_Rear_Light.P_RocketLauncher_MuzzleFlash_Rear_Light" (Transformation|GetActorLocation)))
  (Audio|SpawnSoundAttached "/Game/SciFiWeapLight/Sound/RocketLauncher/Wavs/RL_Fire_ST04.RL_Fire_ST04" _returnvalue "None" "0, 0, 0" "0, 0, 0" "KeepRelativeOffset" false 1.0 1.0 0.0 0 0)
  (Effects|SpawnEmitterAttached "/Game/SciFiWeapLight/FX/Particles/P_RocketLauncher_Trail_Light.P_RocketLauncher_Trail_Light" (Variables|Default|GetSphere) "None" "0, 0, 0" "0, 0, 0" "1.000000,1.000000,1.000000" "KeepRelativeOffset" false)
  (Utilities|FlowControl|Delay 5.0)
  (CallFunction|Explode)
  (Audio|SpawnSoundAttached "/Game/SciFiWeapLight/Sound/RocketLauncher/Wavs/RL_Explosion01.RL_Explosion01" (stale Custom|Explode _returnvalue_2) "None" "0, 0, 0" "0, 0, 0" "KeepRelativeOffset" false 1.0 1.0 0.0 0 0))

(fn ConstructionScript)